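; A VR bow Actor that motion controllers grab, draw and fire.
; The first hand holds the bow, toggling global slow motion off on pickup and on at release; a second hand at the string spawns an attached BP_Arrow.
; Tick turns UI toward the camera and projects the pulling hand onto the bow's axis to move the string.
; Releasing it plays a snap-back timeline that launches the arrow with speed scaled by draw length.
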(event Custom|Shoot
  (Components|Timeline|SetPlayRate (Variables|Default|GetSnapBack) (/ 1.0 0.05))
  (Utilities|FlowControl|Sequence
    (:then_0
      (Utilities|FlowControl|DoOnce false :!label _label
        (:Completed
          (Audio|PlaySound2D "/Game/AProject/Blueprints/Shhoot.Shhoot" 1.0 1.0 0.0 0 0))))
    (:then_1
      (bind _newtrack0 (Timeline|SnapBack PlayFromStart)
        (:Update
          (Transformation|SetRelativeLocation (Variables|Default|GetString) (Math|Vector|Lerp(Vector) (Variables|Default|GetStringRelativeLocation) (Variables|/Script/Engine.SceneComponent|GetRelativeLocation (Variables|Default|GetStringCollision)) _newtrack0) false false)
          (if (> _newtrack0 0.8)
            (bind _arrow (Variables|Default|GetArrow)
              (:then
                (Transformation|DetachFromActor _arrow "KeepWorld" "KeepWorld" "KeepWorld")
                (Default|Shoot _arrow (Math|Float|MapRangeClamped (Variables|Default|GetForceLength) 0.0 6e+01 0.0 3e+03))
                (Actor|Tick|SetActorTickEnabled true)
                (Utilities|FlowControl|Sequence
                  (:then_0
                    (goto _label Reset))
                  (:then_1
                    (Utilities|FlowControl|DoOnce false) ; enters at Reset
                  )))
              (:else))))))))

(event EventTick
  (params (DeltaSeconds :type Float%20%28single-precision%29))
  (bind _grabui (Variables|Default|GetGrabUI))
  (Utilities|FlowControl|Sequence
    (:then_0
      (bind _returnvalue (Actor|GetActorOfClass "/Game/AProject/Blueprints/Player/MotionControllerPawn.MotionControllerPawn_C"))
      (Utilities|IsValid (Variables|/Game/AProject/Blueprints/Player/MotionControllerPawn.MotionControllerPawn_C|GetCamera _returnvalue)
        (:Is%20Valid
          (Transformation|SetWorldRotation _grabui (Math|Conversions|RotationFromXVector (- (Transformation|GetWorldLocation (Variables|/Game/AProject/Blueprints/Player/MotionControllerPawn.MotionControllerPawn_C|GetCamera _returnvalue)) (Transformation|GetWorldLocation _grabui))) false false)
          (Transformation|SetWorldRotation (Variables|Default|GetGrabUI) (Math|Conversions|RotationFromXVector (- (Transformation|GetWorldLocation (Variables|/Game/AProject/Blueprints/Player/MotionControllerPawn.MotionControllerPawn_C|GetCamera _returnvalue)) (Transformation|GetWorldLocation (Variables|Default|GetWidget)))) false false))))
    (:then_1
      (bind _secondhand (Variables|Default|GetSecondHand)
        (:then
          (Variables|Default|SetStringRelativeLocation (Math|Vector|ProjectVectorontoVector (Math|Transform|InverseTransformLocation (Transformation|GetActorTransform) (Transformation|GetWorldLocation _secondhand)) (Math|Vector|GetRightVector (Variables|/Script/Engine.SceneComponent|GetRelativeRotation (Variables|Debug|GetStaticMeshComponent)))))
          (Variables|Default|SetForceLength (Math|Vector|VectorLength (- (Variables|Default|GetStringRelativeLocation) (Variables|/Script/Engine.SceneComponent|GetRelativeLocation (Variables|Default|GetStringCollision)))))
          (if (and (< (Math|Vector|DotProduct (Math|Vector|Normalize (- (Variables|Default|GetStringRelativeLocation) (Variables|/Script/Engine.SceneComponent|GetRelativeLocation (Variables|Default|GetStringCollision)))) (Math|Vector|GetRightVector (Variables|/Script/Engine.SceneComponent|GetRelativeRotation (Variables|Debug|GetStaticMeshComponent)))) 0.0) (< (Variables|Default|GetForceLength) 6e+01))
            (Transformation|SetRelativeLocation (Variables|Default|GetString) (Variables|Default|GetStringRelativeLocation) false false)))
        (:else)))))

(event EventPickup
  (params (MotionController :type Scene%20Component%20Object%20Reference) (HandMesh :type Scene%20Component%20Object%20Reference))
  (Variables|Default|GetFirstHand
    (:then
      (for _array_element (Collision|GetOverlappingActors (Variables|Default|GetStringCollision) "/Script/Engine.Actor" :!class /Script/Engine.PrimitiveComponent)
        (if (== _array_element (Components|GetOwner MotionController))
          (Variables|Default|SetSecondHand MotionController)
          (bind _returnvalue (Game|SpawnActorfromClass "/Game/AProject/Testing/BP_Arrow.BP_Arrow_C" (Math|Transform|MakeTransform "0, 0, 0" "0, 0, 0" "1.200000,2.500000,2.500000") "AlwaysSpawn" 0 0))
          (bind _output_get (Variables|Default|SetArrow _returnvalue))
          (Transformation|AttachComponentToComponent _output_get (Variables|Default|GetString) "None" "SnapToTarget" "SnapToTarget" "KeepWorld" false)
          (Utilities|FlowControl|DoOnce false
            (:Completed
              (Audio|PlaySound2D "/Game/AProject/Blueprints/Loading.Loading" 1.0 1.0 0.0 0 0))))))
    (:else
      (bind _output_get_2 (Variables|Default|SetFirstHand HandMesh))
      (Transformation|AttachComponentToComponent (Variables|Debug|GetStaticMeshComponent) _output_get_2 "Bow" "SnapToTarget" "SnapToTarget" "KeepWorld" false)
      (Rendering|SetVisibility (Variables|Default|GetGrabUI) false false)
      (Utilities|Time|SetGlobalTimeDilation 1.0))))

(event EventDrop
  (params (MotionController :type Scene%20Component%20Object%20Reference) (HandMesh :type Scene%20Component%20Object%20Reference))
  (bind _secondhand (Variables|Default|GetSecondHand)
    (:then
      (if (== _secondhand MotionController)
        (Variables|Default|SetSecondHand 0)
        (Actor|Tick|SetActorTickEnabled false)
        (CallFunction|Shoot)))
    (:else
      (bind _firsthand (Variables|Default|GetFirstHand)
        (:then
          (if (== _firsthand HandMesh)
            (Transformation|DetachFromActor "KeepWorld" "KeepWorld" "KeepWorld")
            (Variables|Default|SetFirstHand 0)
            (Variables|Default|SetSecondHand 0)
            (Rendering|SetVisibility (Variables|Default|GetGrabUI) true false)
            (Utilities|Time|SetGlobalTimeDilation 0.1)))
        (:else)))))

(fn ConstructionScript)