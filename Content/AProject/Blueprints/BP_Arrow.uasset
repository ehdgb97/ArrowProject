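; BP_Arrow is an arrow projectile that stops on its first overlap, plays a material effect and destroys itself.
; Shoot launches it along local X at a given velocity and enables query-only collision.
; On overlap it disables movement and collision, then sets a dynamic material's Location ahead of the actor.
; A timeline, separate for BP_Enemy and other actors, animates the Amount parameter before destruction; no damage is applied here.
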(event OnComponentBeginOverlap(ArrowColl)
  (params (OverlappedComponent :type Primitive%20Component%20Object%20Reference) (OtherActor :type Actor%20Object%20Reference) (OtherComp :type Primitive%20Component%20Object%20Reference) (OtherBodyIndex :type Integer) (bFromSweep :type Boolean) (SweepResult :type Hit%20Result%20Structure%20%28by%20ref%29))
  (bind _projectilemovement (Variables|Default|GetProjectileMovement))
  (bind _newvar_0 (Variables|Default|GetNewVar_0))
  (bind _newvar_0_2 (Variables|Default|GetNewVar_0))
  (bind _projectilemovement_2 (Variables|Default|GetProjectileMovement))
  (Utilities|Casting|CastToBP_Enemy OtherActor
    (:then
      (Components|Movement|StopMovementImmediately _projectilemovement)
      (Components|Activation|SetActive _projectilemovement false false)
      (Collision|SetCollisionEnabled (Variables|Default|GetArrow%20Coll) "NoCollision")
      (Rendering|Material|SetVectorParameterValue _newvar_0 "Location" (Math|Conversions|ToLinearColor(Vector) (+ (Transformation|GetActorLocation) (* (Transformation|GetActorForwardVector) 85.0))) :!class /Script/Engine.MaterialInstanceDynamic)
      (bind _newtrack_0 (Timeline|Timeline_0 PlayFromStart)
        (:Update
          (Rendering|Material|SetScalarParameterValue _newvar_0 "Amount" _newtrack_0 :!class /Script/Engine.MaterialInstanceDynamic))
        (:Finished
          (Actor|DestroyActor))))
    (:CastFailed
      (Components|Movement|StopMovementImmediately _projectilemovement_2)
      (Components|Activation|SetActive _projectilemovement_2 false false)
      (Collision|SetCollisionEnabled (Variables|Default|GetArrow%20Coll) "NoCollision")
      (Rendering|Material|SetVectorParameterValue _newvar_0_2 "Location" (Math|Conversions|ToLinearColor(Vector) (+ (Transformation|GetActorLocation) (* (Transformation|GetActorForwardVector) 85.0))) :!class /Script/Engine.MaterialInstanceDynamic)
      (bind _newtrack_0_2 (Timeline|Timeline_1 PlayFromStart)
        (:Update
          (Rendering|Material|SetScalarParameterValue _newvar_0_2 "Amount" _newtrack_0_2 :!class /Script/Engine.MaterialInstanceDynamic))
        (:Finished
          (Actor|DestroyActor))))))

(event OnComponentHit(ArrowColl)
  (params (HitComponent :type Primitive%20Component%20Object%20Reference) (OtherActor :type Actor%20Object%20Reference) (OtherComp :type Primitive%20Component%20Object%20Reference) (NormalImpulse :type Vector :default "0, 0, 0") (Hit :type Hit%20Result%20Structure%20%28by%20ref%29)))

(event Custom|Shoot
  (params (Velocity :type Float%20%28single-precision%29))
  (bind _projectilemovement (Variables|Default|GetProjectileMovement))
  (bind _output_get (Variables|/Script/Engine.ProjectileMovementComponent|SetInitialSpeed _projectilemovement Velocity))
  (Variables|/Script/Engine.ProjectileMovementComponent|SetMaxSpeed _projectilemovement _output_get)
  (Game|Components|ProjectileMovement|SetVelocityinLocalSpace _projectilemovement (Math|Vector|MakeVector Velocity 0.0 0.0))
  (Components|Activation|SetActive (Variables|Default|GetProjectileMovement) true true)
  (Collision|SetCollisionEnabled (Variables|Default|GetArrow%20Coll) "QueryOnly"))

(event EventBeginPlay
  (bind _returnvalue (Rendering|Material|CreateDynamicMaterialInstance (Variables|Debug|GetStaticMeshComponent) 0 0 "None" :!class /Script/Engine.PrimitiveComponent))
  (Variables|Default|SetNewVar_0 _returnvalue))

(fn ConstructionScript)