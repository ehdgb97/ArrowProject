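; BP_Enemy is an enemy actor that plays a material effect when hit by a BP_Arrow, then destroys itself.
; BeginPlay creates a dynamic material instance on the Cube mesh.
; An arrow overlap writes the arrow component's world location to the material's Location parameter and disables Cube collision.
; A timeline then animates the Amount parameter from that hit and destroys the actor when finished.
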(event OnComponentBeginOverlap(Cube)
  (params (OverlappedComponent :type Primitive%20Component%20Object%20Reference) (OtherActor :type Actor%20Object%20Reference) (OtherComp :type Primitive%20Component%20Object%20Reference) (OtherBodyIndex :type Integer) (bFromSweep :type Boolean) (SweepResult :type Hit%20Result%20Structure%20%28by%20ref%29))
  (Utilities|Casting|CastToBP_Arrow OtherActor)
  (Rendering|Material|SetVectorParameterValue (Variables|Default|GetNewVar_0) "Location" (Math|Conversions|ToLinearColor(Vector) (Transformation|GetWorldLocation OtherComp)) :!class /Script/Engine.MaterialInstanceDynamic)
  (Collision|SetCollisionEnabled (Variables|Default|GetCube) "NoCollision")
  (bind _newtrack_0 (Timeline|Timeline_0 PlayFromStart)
    (:Update
      (Rendering|Material|SetScalarParameterValue (Variables|Default|GetNewVar_0) "Amount" _newtrack_0 :!class /Script/Engine.MaterialInstanceDynamic))
    (:Finished
      (Actor|DestroyActor))))

(event EventBeginPlay
  (bind _returnvalue (Rendering|Material|CreateDynamicMaterialInstance (Variables|Default|GetCube) 0 0 "None" :!class /Script/Engine.PrimitiveComponent))
  (Variables|Default|SetNewVar_0 _returnvalue))

(fn ConstructionScript)