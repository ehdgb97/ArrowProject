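; Grabbable lever switch for a stair puzzle that toggles StairA and StairC between flying and landed.
; While held, Tick pitches the lever toward a proxy Cube within a clamped angle computed in Angle's local space.
; Capsule-Box overlap fires both toggles once, releases the grab, animates the lever and snaps the Cube to the Arrow.
; A game mode flag blocks switch use until a delayed reset.
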(event Custom|Reset
  (bind _as_bp_puzzle_gamemode (Variables|Default|GetAs%20BP%20Puzzle%20Gamemode))
  (bind _stairc (Variables|Default|GetStairC))
  (bind _staira (Variables|Default|GetStairA))
  (Utilities|FlowControl|Sequence
    (:then_0
      (Utilities|FlowControl|DoOnce false) ; enters at Reset
    )
    (:then_1
      (Utilities|FlowControl|DoOnce false) ; enters at Reset
    )))

(event EventBeginPlay
  (bind _cube (Variables|Default|GetCube))
  (Variables|Default|SetLeverRelativeRotation (Variables|/Script/Engine.SceneComponent|GetRelativeRotation (Variables|Default|GetLever)))
  (Variables|Default|SetGrabRelativeLocation (Variables|/Script/Engine.SceneComponent|GetRelativeLocation _cube))
  (Variables|Default|SetGrabRelativeRotation (Variables|/Script/Engine.SceneComponent|GetRelativeRotation _cube))
  (bind _returnvalue (Actor|GetActorOfClass "/Game/AProject/Testing/BP_StairA.BP_StairA_C"))
  (Variables|Default|SetStairA _returnvalue)
  (bind _returnvalue_2 (Actor|GetActorOfClass "/Game/AProject/Testing/BP_StairB.BP_StairB_C"))
  (Variables|Default|SetStairB _returnvalue_2)
  (bind _returnvalue_3 (Actor|GetActorOfClass "/Game/AProject/Testing/BP_StairC.BP_StairC_C"))
  (Variables|Default|SetStairC _returnvalue_3)
  (bind _returnvalue_4 (Actor|GetActorOfClass "/Game/AProject/Testing/BP_StairD.BP_StairD_C"))
  (Variables|Default|SetStairD _returnvalue_4)
  (bind _asbp_puzzle_gamemode (Utilities|Casting|CastToBP_PuzzleGamemode (Game|GetGameMode)))
  (Variables|Default|SetAs%20BP%20Puzzle%20Gamemode _asbp_puzzle_gamemode))

(event EventTick
  (params (DeltaSeconds :type Float%20%28single-precision%29))
  (bind _lever (Variables|Default|GetLever))
  (bind _angle (Variables|Default|GetAngle))
  (bind _angle_2 (Variables|Default|GetAngle))
  (bind _cube (Variables|Default|GetCube))
  (bind _as_bp_puzzle_gamemode (Variables|Default|GetAs%20BP%20Puzzle%20Gamemode))
  (bind _stairc (Variables|Default|GetStairC))
  (bind _staira (Variables|Default|GetStairA))
  (bind _returnvalue (Math|Vector|GetUpVector _angle))
  (bind _returnvalue_2 (Transformation|GetWorldLocation _cube))
  (bind _returnvalue_3 (Transformation|GetWorldTransform _angle_2))
  (bind _relativerotation (Variables|/Script/Engine.SceneComponent|GetRelativeRotation _lever))
  (bind _returnvalue_4 (Math|Transform|InverseTransformLocation _returnvalue_3 _returnvalue_2))
  (bind _returnvalue_5 (Math|Vector|MakeVector (.x _returnvalue_4) 0.0 (.z _returnvalue_4)))
  (bind _returnvalue_6 (Math|Vector|Normalize _returnvalue_5))
  (if (not (Variables|/Game/AProject/Testing/BP_PuzzleGamemode.BP_PuzzleGamemode_C|GetIsSwitchPlayed? (Variables|Default|GetAs%20BP%20Puzzle%20Gamemode)))
    (if (Class|PrimitiveComponent|IsOverlappingComponent (Variables|Default|GetCapsule) (Variables|Default|GetBox))
      (Utilities|FlowControl|Sequence
        (:then_0
          (Utilities|FlowControl|DoOnce false
            (:Completed
              (if (Variables|/Game/AProject/Testing/BP_StairA.BP_StairA_C|GetIsA_Flyed _staira)
                (Default|Land _staira)
                (else
                  (Default|Fly _staira))))))
        (:then_1
          (Utilities|FlowControl|DoOnce false
            (:Completed
              (if (Variables|/Game/AProject/Testing/BP_StairC.BP_StairC_C|GetIsC_Flyed _stairc)
                (Default|Land _stairc)
                (else
                  (Default|Fly _stairc)))))))
      (Variables|/Game/AProject/Testing/BP_PuzzleGamemode.BP_PuzzleGamemode_C|SetIsSwitchPlayed? _as_bp_puzzle_gamemode true)
      (Default|TryRelease (Variables|Default|GetGrabComponent))
      (Components|MoveComponentTo (Variables|Default|GetLever) "0,2.000000,70.000000" "0, 0,90.000000" false false 1.0 true)
      (Transformation|SetWorldLocation (Variables|Default|GetCube) (Transformation|GetWorldLocation (Variables|Default|GetArrow)) false false)
      (Utilities|FlowControl|Delay 1.0)
      (Variables|/Game/AProject/Testing/BP_PuzzleGamemode.BP_PuzzleGamemode_C|SetIsSwitchPlayed? _as_bp_puzzle_gamemode false)
      (CallFunction|Reset)
      (else
        (Transformation|SetRelativeRotation (Variables|Default|GetLever) (Math|Rotator|MakeRotator (.roll _relativerotation) (Math|Float|Clamp(Float) (* (Class|KismetMathLibrary|DegAcos (Math|Vector|DotProduct _returnvalue_6 _returnvalue)) (Math|Float|Sign(Float) (.y (Math|Vector|CrossProduct _returnvalue_6 _returnvalue)))) 0.0 6e+01) (.yaw _relativerotation)) false false)))))

(event EventPick
  (params (Attach%20to :type Scene%20Component%20Object%20Reference))
  (if (Variables|/Game/AProject/Testing/BP_PuzzleGamemode.BP_PuzzleGamemode_C|GetIsSwitchPlayed? (Variables|Default|GetAs%20BP%20Puzzle%20Gamemode))
    (Default|TryRelease (Variables|Default|GetGrabComponent))
    (else
      (Actor|Tick|SetActorTickEnabled true))))

(event EventDrop
  (params (Attach :type Scene%20Component%20Object%20Reference))
  (Transformation|SetWorldLocation (Variables|Default|GetCube) (Transformation|GetWorldLocation (Variables|Default|GetArrow)) false false)
  (Actor|Tick|SetActorTickEnabled false))

(fn ConstructionScript)