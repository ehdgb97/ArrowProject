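; BP_TestBow is a test bow actor drawn with a secondary hand grab, which fires a BP_Arrow on release.
; Grabbing spawns an arrow on the string and enables Tick, which projects the hand onto the bow's local axis to move the string within a limited draw range.
; Release plays a quick SnapBack timeline that returns the string, then near its end detaches the arrow and shoots it with strength mapped from draw length.
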(event Custom|Shoot
  (Components|Timeline|SetPlayRate (Variables|Default|GetSnapBack) (/ 1.0 0.05))
  (Utilities|FlowControl|Sequence
    (:then_0
      (Audio|PlaySound2D "/Game/AProject/Blueprints/Shhoot.Shhoot" 1.0 1.0 0.0 0 0))
    (:then_1
      (bind _newtrack0 (Timeline|SnapBack PlayFromStart)
        (:Update
          (Transformation|SetRelativeLocation (Variables|Default|GetString) (Math|Vector|Lerp(Vector) (Variables|Default|GetStringRelativeLocation) (Variables|/Script/Engine.SceneComponent|GetRelativeLocation (Variables|Default|GetStringCollision)) _newtrack0) false false)
          (if (> _newtrack0 0.8)
            (bind _arrow (Variables|Default|GetArrow)
              (:then
                (Transformation|DetachFromActor _arrow "KeepWorld" "KeepWorld" "KeepWorld")
                (Default|Shoot (Variables|Default|GetArrow) (Math|Float|MapRangeClamped (Variables|Default|GetForceLength) 0.0 6e+01 0.0 3e+03)))
              (:else))))))))

(event EventSecondaryGrabPressed
  (params (Hand :type Scene%20Component%20Object%20Reference))
  (Variables|Default|SetSecondHand Hand)
  (Actor|Tick|SetActorTickEnabled true)
  (bind _returnvalue (Game|SpawnActorfromClass "/Game/AProject/Testing/BP_Arrow.BP_Arrow_C" (Math|Transform|MakeTransform "0, 0, 0" "0, 0, 0" "1.200000,2.500000,2.500000") "AlwaysSpawn" 0 0))
  (bind _output_get (Variables|Default|SetArrow _returnvalue))
  (Transformation|AttachComponentToComponent _output_get (Variables|Default|GetString) "None" "SnapToTarget" "SnapToTarget" "KeepWorld" false)
  (Audio|PlaySound2D "/Game/AProject/Blueprints/Loading.Loading" 1.0 1.0 0.0 0 0))

(event EventSecondaryGrabReleased
  (params (Hand :type Scene%20Component%20Object%20Reference))
  ;[1 1 1] 활을 놓았을 때
  (Variables|Default|SetSecondHand 0)
  (Actor|Tick|SetActorTickEnabled false)
  (CallFunction|Shoot))

(event EventTick
  (params (DeltaSeconds :type Float%20%28single-precision%29))
  (bind _secondhand (Variables|Default|GetSecondHand)
    (:then
      (Variables|Default|SetStringRelativeLocation (Math|Vector|ProjectVectorontoVector (Math|Transform|InverseTransformLocation (Transformation|GetActorTransform) (Transformation|GetWorldLocation _secondhand)) (Math|Vector|GetRightVector (Variables|/Script/Engine.SceneComponent|GetRelativeRotation (Variables|Debug|GetStaticMeshComponent)))))
      (Variables|Default|SetForceLength (Math|Vector|VectorLength (- (Variables|Default|GetStringRelativeLocation) (Variables|/Script/Engine.SceneComponent|GetRelativeLocation (Variables|Default|GetStringCollision)))))
      (if (and (< (Math|Vector|DotProduct (Math|Vector|Normalize (- (Variables|Default|GetStringRelativeLocation) (Variables|/Script/Engine.SceneComponent|GetRelativeLocation (Variables|Default|GetStringCollision)))) (Math|Vector|GetRightVector (Variables|/Script/Engine.SceneComponent|GetRelativeRotation (Variables|Debug|GetStaticMeshComponent)))) 0.0) (< (Variables|Default|GetForceLength) 6e+01))
        (Transformation|SetRelativeLocation (Variables|Default|GetString) (Variables|Default|GetStringRelativeLocation) false false)))
    (:else)))

(fn ConstructionScript)