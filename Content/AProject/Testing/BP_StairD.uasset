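; BP_StairD is a test stair actor that moves vertically through two custom events, Fly and Land.
; Each event sets the IsDFlyed flag, stores the current location as a start point, then plays its own height timeline from the start.
; Every timeline update offsets Z from that start location, adding for Fly and subtracting for Land, while X and Y stay fixed.
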(event Custom|Land
  (Variables|Default|SetIsD_Flyed false)
  (Variables|Default|SetStartLocation (Transformation|GetActorLocation))
  (bind _height (Timeline|LandHeight PlayFromStart)
    (:Update
      (Transformation|SetActorLocation (Math|Vector|MakeVector (.x (Variables|Default|GetStartLocation)) (.y (Variables|Default|GetStartLocation)) (- (.z (Variables|Default|GetStartLocation)) _height)) false false))))

(event Custom|Fly
  (Variables|Default|SetIsD_Flyed true)
  (Variables|Default|SetStartLocation (Transformation|GetActorLocation))
  (bind _height (Timeline|FlyHeight PlayFromStart)
    (:Update
      (Transformation|SetActorLocation (Math|Vector|MakeVector (.x (Variables|Default|GetStartLocation)) (.y (Variables|Default|GetStartLocation)) (+ (.z (Variables|Default|GetStartLocation)) _height)) false false))))

(event EventBeginPlay)

(event Collision|EventActorBeginOverlap
  (params (OtherActor :type Actor%20Object%20Reference)))

(event EventTick
  (params (DeltaSeconds :type Float%20%28single-precision%29)))

(fn ConstructionScript)