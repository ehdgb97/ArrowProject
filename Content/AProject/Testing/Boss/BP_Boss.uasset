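; Test boss actor that takes damage while attackable and fires projectile volleys, with unfinished attack logic.
; Tick drives a state machine: Idle spawns a shield and enters Attack, while Rest disables damage and returns to Idle.
; Attack waits out an animation wind-up, then spawns up to eight randomly rolled projectiles at the Fire component.
; WatchTarget is empty, and the switch to Rest and the pizza area-attack chain are disconnected.
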(event Custom|Attack
  (params (DeltaSeconds :type Float%20%28single-precision%29))
  ;[1 1 1] 피자
  ;;[1 1 1] Enum으로 대체가능?
  (Variables|Animate|Bool|SetbAttack_Ani true)
  ;;[1 1 1] 공격 준비 블랜딩타임
  (bind _output_get (Variables|Default|SetAttack_Blend_Time (+ (Variables|Default|GetAttack_Blend_Time) (Utilities|Time|GetWorldDeltaSeconds))))
  (if (> _output_get (Variables|Default|GetAttackStart))
    ;;[1 1 1] 발사횟수_alpha 피없을 때 횟수증가
    (if (not (== (Variables|Default|GetFireTime) 8))
      (Utilities|FlowControl|Delay 0.1)
      (Game|SpawnActorfromClass "/Game/AProject/Testing/Boss/BP_BossProjectile.BP_BossProjectile_C" (Math|Transform|MakeTransform (Transformation|GetWorldLocation (Variables|Default|GetFire)) (Math|Rotator|MakeRotator (Math|Random|RandomFloatinRange 6e+01 8e+01) (.pitch (Transformation|GetActorRotation)) 0.0) "1,1,1") "AlwaysSpawn" 0 0)
      (Variables|Default|SetFireTime (+ (Variables|Default|GetFireTime) 1)))
    (else
      ;;[1 1 1] 쳐다보기 정면으로 셋팅하기
      (Utilities|FlowControl|DoOnce false
        (:Completed
          (CallFunction|WatchTarget))))))

(event EventBeginPlay
  (Variables|Default|SetHealth (Variables|Default|GetMax_HP)))

(event Collision|EventActorBeginOverlap
  (params (OtherActor :type Actor%20Object%20Reference)))

(event EventTick
  (params (DeltaSeconds :type Float%20%28single-precision%29))
  (switch Utilities|FlowControl|Switch|SwitchonBoss_Enum (Variables|Default|GetBoss_State)
    (:NewEnumerator0
      (Game|SpawnActorfromClass "/Game/AProject/Testing/Boss/BP_Shield.BP_Shield_C" (Math|Transform|MakeTransform "0, 0, 0" "0, 0, 0" "1,1,1") "Undefined" 0 0)
      (Variables|Default|SetBoss_State "NewEnumerator1"))
    (:NewEnumerator1
      (CallFunction|Attack 0.0))
    (:NewEnumerator2
      (Variables|Animate|Bool|SetbRest_Ani true)
      (Variables|Default|SetbIsAttackable? false)
      (Variables|Default|SetBoss_State "NewEnumerator0"))))

(event Game|Damage|EventAnyDamage
  (params (Damage :type Float%20%28single-precision%29) (DamageType :type Damage%20Type%20Object%20Reference) (InstigatedBy :type Controller%20Object%20Reference) (DamageCauser :type Actor%20Object%20Reference))
  (if (Variables|Default|GetbIsAttackable?)
    (Variables|Default|SetbDamaged true)
    (Variables|Default|SetHealth (- (Variables|Default|GetHealth) Damage))))

(fn ConstructionScript)

(fn WatchTarget)