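; BP_StairB is a stair actor in a testing folder that slides between positions when its Fly and Land events are called.
; Each event records the current location as a start point, then plays its own timeline (FlyHeight or LandHeight) to offset the actor from it.
; Despite the height naming, the offset is on the Y axis, added for Fly and subtracted for Land.
; IsBFlyed tracks the state but is never read here.
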(event Custom|Land
  (Variables|Default|SetIsB_Flyed false)
  (Variables|Default|SetStartLocation (Transformation|GetActorLocation))
  (bind _height (Timeline|LandHeight PlayFromStart)
    (:Update
      (Transformation|SetActorLocation (Math|Vector|MakeVector (.x (Variables|Default|GetStartLocation)) (- (.y (Variables|Default|GetStartLocation)) _height) (.z (Variables|Default|GetStartLocation))) false false))))

(event Custom|Fly
  (Variables|Default|SetIsB_Flyed true)
  (Variables|Default|SetStartLocation (Transformation|GetActorLocation))
  (bind _height (Timeline|FlyHeight PlayFromStart)
    (:Update
      (Transformation|SetActorLocation (Math|Vector|MakeVector (.x (Variables|Default|GetStartLocation)) (+ (.y (Variables|Default|GetStartLocation)) _height) (.z (Variables|Default|GetStartLocation))) false false))))

(event EventBeginPlay)

(event Collision|EventActorBeginOverlap
  (params (OtherActor :type Actor%20Object%20Reference)))

(event EventTick
  (params (DeltaSeconds :type Float%20%28single-precision%29)))

(fn ConstructionScript)