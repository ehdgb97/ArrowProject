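; BP_Switch1 is a lever switch whose pitch follows the position of its Cube component.
; Pick and Drop events turn actor tick on and off.
; Each tick derives a signed, clamped angle from Cube's X-Z offset in Angle's local space against Angle's world up vector, using dot and cross products.
; Tick also prints a debug string while Capsule overlaps Box, with no other switch action.
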(event EventBeginPlay)

(event Collision|EventActorBeginOverlap
  (params (OtherActor :type Actor%20Object%20Reference)))

(event EventTick
  (params (DeltaSeconds :type Float%20%28single-precision%29))
  (bind _lever (Variables|Default|GetLever))
  (bind _angle (Variables|Default|GetAngle))
  (bind _angle_2 (Variables|Default|GetAngle))
  (bind _cube (Variables|Default|GetCube))
  (bind _returnvalue (Math|Vector|GetUpVector _angle))
  (bind _returnvalue_2 (Transformation|GetWorldLocation _cube))
  (bind _returnvalue_3 (Transformation|GetWorldTransform _angle_2))
  (bind _relativerotation (Variables|/Script/Engine.SceneComponent|GetRelativeRotation _lever))
  (bind _returnvalue_4 (Math|Transform|InverseTransformLocation _returnvalue_3 _returnvalue_2))
  (bind _returnvalue_5 (Math|Vector|MakeVector (.x _returnvalue_4) 0.0 (.z _returnvalue_4)))
  (bind _returnvalue_6 (Math|Vector|Normalize _returnvalue_5))
  (Utilities|FlowControl|Sequence
    (:then_0
      (if (Class|PrimitiveComponent|IsOverlappingComponent (Variables|Default|GetCapsule) (Variables|Default|GetBox))
        (Development|PrintString "Hello")))
    (:then_1
      (Transformation|SetRelativeRotation (Variables|Default|GetLever) (Math|Rotator|MakeRotator (.roll _relativerotation) (Math|Float|Clamp(Float) (* (Class|KismetMathLibrary|DegAcos (Math|Vector|DotProduct _returnvalue_6 _returnvalue)) (Math|Float|Sign(Float) (.y (Math|Vector|CrossProduct _returnvalue_6 _returnvalue)))) 0.0 6e+01) (.yaw _relativerotation)) false false))))

(event EventPick
  (params (Attach%20to :type Scene%20Component%20Object%20Reference))
  (Actor|Tick|SetActorTickEnabled true))

(event EventDrop
  (params (Attach :type Scene%20Component%20Object%20Reference))
  (Actor|Tick|SetActorTickEnabled false))

(fn ConstructionScript)