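; VR pickup actor that acts as a lever switch, with a grabbable Cube that drives the Lever's tilt.
; Pickup attaches only the Cube to the motion controller passed in by BP_MotionController.
; Each Tick adds the world X offset between Arrow and Cube to the Lever's pitch, clamped to a symmetric range.
; Drop enables physics on StaticMeshComponent and detaches the actor, rather than detaching the Cube itself.
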(event EventBeginPlay)

(event Collision|EventActorBeginOverlap
  (params (OtherActor :type Actor%20Object%20Reference)))

(event EventTick
  (params (DeltaSeconds :type Float%20%28single-precision%29))
  (bind _lever (Variables|Default|GetLever))
  (bind _returnvalue (Transformation|GetWorldRotation _lever))
  (Transformation|SetWorldRotation _lever (Math|Rotator|MakeRotator (.roll _returnvalue) (Math|Float|Clamp(Float) (+ (.pitch _returnvalue) (.x (- (Transformation|GetWorldLocation (Variables|Default|GetArrow)) (Transformation|GetWorldLocation (Variables|Default|GetCube))))) -6e+01 6e+01) (.yaw _returnvalue)) false false))

(event EventPickup
  (params (MotionController :type Scene%20Component%20Object%20Reference) (HandMesh :type Scene%20Component%20Object%20Reference))
  (Transformation|AttachComponentToComponent (Variables|Default|GetCube) MotionController "None" "KeepRelative" "KeepRelative" "KeepRelative" true))

(event EventDrop
  (params (MotionController :type Scene%20Component%20Object%20Reference) (HandMesh :type Scene%20Component%20Object%20Reference))
  (Physics|SetSimulatePhysics (Variables|Debug|GetStaticMeshComponent) true)
  (Transformation|DetachFromActor "KeepWorld" "KeepWorld" "KeepWorld"))

(fn ConstructionScript)